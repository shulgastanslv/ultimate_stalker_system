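; BP_ItemObject is an inventory item object that exposes its data through simple getter functions.
; Most getters read the ItemDetails struct for identity, dimensions, weight, count, condition, icons and sounds, while outfit characteristics and max weight come from OutfitStats.
; GetIcon picks the normal or rotated icon from the Rotated flag, and returns no icon unless both are valid.
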(fn `GetCondition`
  (returns (Condition :type "Float (double-precision)"))
  (return (`.Condition_9_F1E48C43492D4DFA23A390917655D46F` (break `/Game/Inventory/Structures/S_ItemDetails` (`self.ItemDetails`)))))

(fn `GetCount`
  (returns (Count :type Integer))
  (return (`.Count_10_36121AE344382FC4B8EFFE9D8099ABBA` (break `/Game/Inventory/Structures/S_ItemDetails` (`self.ItemDetails`)))))

(fn `GetDimensions`
  (returns (Dimensions :type "IntPoint Structure"))
  (return (`.Dimensions_41_F223E7E24BC38750C8CBFE9580E7807E` (break `/Game/Inventory/Structures/S_ItemDetails` (`self.ItemDetails`)))))

(fn `GetDropSound`
  (returns (DropSound :type "SoundCue Object Reference"))
  (return (`.Drop_64_D80530714D71DD75B9500492D6492C28` (break `/Game/Inventory/Structures/S_ItemDetails` (`self.ItemDetails`)))))

(fn `GetEquipmentSound`
  (returns (EquipmentSound :type "SoundCue Object Reference"))
  (return (`.Equipment_65_5C8FA5154A24328653633B969079FB7A` (break `/Game/Inventory/Structures/S_ItemDetails` (`self.ItemDetails`)))))

(fn `GetIcon`
  (returns (Icon :type "MaterialInterface Object Reference"))
  (bind ((`ID_69_A97F860C4B8ABAF2864DFFBBB2C4BD45` _id) (`Icon_38_E9A591FF4B94A98426E42889CA56B19A` _icon) (`IconRatated_39_D5175E2B44327E0F26F894811C6A976A` _iconratated) (`Rotated?_44_2296B3EC48C04BCC8D2921AD05648AE4` _rotated_)) (break `/Game/Inventory/Structures/S_ItemDetails` (`self.ItemDetails`)))
  (`/Engine/EditorBlueprintResources/StandardMacros.IsValid` _icon
    (:`Is Valid`
      (`/Engine/EditorBlueprintResources/StandardMacros.IsValid` _iconratated
        (:`Is Valid`
          (return (select `bool` _rotated_ :`false` _icon :`true` _iconratated)))
        (:`Is Not Valid`
          (return null))))
    (:`Is Not Valid`
      (return null))))

(fn `GetItemClass`
  (returns (`Item Class` :type "/Game/Inventory/Blueprints/BP_MasterItem Class Reference"))
  (return (`.ItemClass_29_A4EF3F8145ED620C8201EFBC885E8E31` (break `/Game/Inventory/Structures/S_ItemDetails` (`self.ItemDetails`)))))

(fn `GetItemDetails`
  (returns (S_ItemDetails :type "/Game/Inventory/Structures/S_ItemDetails Structure"))
  (return (`self.ItemDetails`)))

(fn `GetItemType`
  (returns (`Item Type` :type "/Game/Inventory/Enumerations/E_ItemType Enum"))
  (return (`.ItemType_16_43F3566046E9FC45FE20E3A9C50CF57D` (break `/Game/Inventory/Structures/S_ItemDetails` (`self.ItemDetails`)))))

(fn `GetMaxWeight`
  (returns (MaxWeight :type "Float (double-precision)"))
  (return (`.MaxWeight_3_02A2189A49221E69A2D88CA76B17A1F8` (break `/Game/Inventory/Structures/S_OutfitStats` (`self.OutfitStats`)))))

(fn `GetName`
  (returns (Name :type Name))
  (return (`.Name_2_CF0C1F604F2013B008F5E2A19F47D3A7` (break `/Game/Inventory/Structures/S_ItemDetails` (`self.ItemDetails`)))))

(fn `GetOutfitCharacteristics`
  (returns (S_OutfitCharacteristics :type "/Game/Inventory/Structures/S_OutfitStats Structure"))
  (return (`self.OutfitStats`)))

(fn `GetRotationIcon`
  (returns (`Icon Ratated` :type "MaterialInterface Object Reference"))
  (return (`.IconRatated_39_D5175E2B44327E0F26F894811C6A976A` (break `/Game/Inventory/Structures/S_ItemDetails` (`self.ItemDetails`)))))

(fn `GetSoundOfUse`
  (returns (SoundOfUse :type "SoundCue Object Reference"))
  (return (`.SoundOfUse_60_84DE22704E5FD4DAD16184AA2B078293` (break `/Game/Inventory/Structures/S_ItemDetails` (`self.ItemDetails`)))))

(fn `GetWeight`
  (returns (Weight :type "Float (double-precision)"))
  (return (`.Weight_13_C5B3DFC44AD68E721B6FAA83A0F876DA` (break `/Game/Inventory/Structures/S_ItemDetails` (`self.ItemDetails`)))))