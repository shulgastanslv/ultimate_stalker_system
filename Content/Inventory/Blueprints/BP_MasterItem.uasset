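; BP_MasterItem is an inventory item Blueprint that holds an ItemObject, apparently as the base for specific items.
; On BeginPlay it fills ItemObject from GetDefaultItemObject when none is valid, so an already assigned object is kept.
; GetDefaultItemObject returns nothing here, which suggests child Blueprints override it to supply their own item.
; GetItem exposes the stored ItemObject to callers.
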(event `self.ReceiveBeginPlay`
  (if (not (`KismetSystemLibrary.IsValid` (`self.Item Object`)))
    (bind _item_object (`self.GetDefaultItemObject`))
    (set `self.Item Object` _item_object)))

(fn `GetDefaultItemObject`
  (returns (`Item Object` :type "/Game/Inventory/BP_ItemObject Object Reference"))
  (return null))

(fn `GetItem`
  (returns (`Item Object` :type "/Game/Inventory/BP_ItemObject Object Reference"))
  (return (`self.Item Object`)))

(fn `UserConstructionScript`)